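; Blueprint Interface for the rune system, declaring the calls that rune widgets and other objects make on whatever implements it.
; It covers moving, swapping and unlocking runes, changing or reading stats, and spending attribute points.
; It also exposes level, experience, gold and spirit queries, plus toggles for the shop widget, mouse input and move-input ignoring, and a main widget getter.
; All functions are empty signatures, so implementers supply the behavior.
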(fn `ChangeStats`
  (params (Stats :type "Array of /Game/RunesSystem/Blueprints/Structures/ST_Stats Structure") (`Subtract?` :type Boolean)))

(fn `GetCurrentExp`
  (returns (CurrentExp :type Integer))
  (return 0))

(fn `GetGold`
  (returns (Gold :type "Float (double-precision)"))
  (return 0.0))

(fn `GetMainWidget`
  (returns (Widget :type "/Game/RunesSystem/Widgets/WBP_MainWidget Object Reference"))
  (return null))

(fn `GetNeededExp`
  (returns (NeededExp :type Integer))
  (return 0))

(fn `GetPlayerLevel`
  (returns (Level :type Integer))
  (return 0))

(fn `GetRequiredSpirits`
  (returns (RequiredSpirits :type Integer))
  (return 0))

(fn `GetSpirits`
  (returns (Spirits :type Integer))
  (return 0))

(fn `GetStats`
  (returns (Stats :type "Array of /Game/RunesSystem/Blueprints/Structures/ST_Stats Structure"))
  (return))

(fn `MoveRune`
  (params (RuneSlotWidget :type "/Game/RunesSystem/Widgets/WBP_RuneSlot Object Reference") (RuneWidget :type "/Game/RunesSystem/Widgets/WBP_Rune Object Reference") (`DroppedInRuneWidget?` :type Boolean)))

(fn `ReceiveExperience`
  (params (Amount :type Integer)))

(fn `SpendAttributePoints`
  (params (Attribute :type "/Game/RunesSystem/Blueprints/Structures/ST_Attributes Structure") (Pts :type Integer)))

(fn `SwapRunes`
  (params (RuneSlotWidget :type "/Game/RunesSystem/Widgets/WBP_RuneSlot Object Reference") (RuneWidget :type "/Game/RunesSystem/Widgets/WBP_Rune Object Reference") (`DroppedInRuneWidget?` :type Boolean)))

(fn `ToggleMouseInput`)

(fn `ToggleMoveIqnoreInput`
  (params (`CanMove?` :type Boolean)))

(fn `ToggleShopWidgetVisibility`
  (params (RunesToSell :type "Array of Name")))

(fn `UnlockRune`
  (params (Rune :type "/Game/RunesSystem/Blueprints/Structures/ST_Rune Structure")))