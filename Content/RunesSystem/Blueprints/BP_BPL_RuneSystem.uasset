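; Blueprint function library of shared helpers for the rune system and its UI.
; Runes are looked up in DT_Runes and count as valid with an ID, icon and stats.
; Searches scan the main widget for an empty rune widget of matching type to return to, or an empty slot matching type and player level.
; Small helpers cover the player character cast, type colors, type matching and a constant spirit formula type.
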(fn `GetDatatableRune`
  (params (Rune :type Name))
  (returns (FoundRune :type "/Game/RunesSystem/Blueprints/Structures/ST_Rune Structure"))
  (bind _returnvalue (`|GetDataTableRow` "/Game/RunesSystem/Blueprints/Datatables/DT_Runes.DT_Runes" Rune)
    (:`then`
      (return _returnvalue))
    (:`RowNotFound`
      (return))))

(fn `GetEmptyRune`
  (params (RuneType :type "/Game/RunesSystem/Blueprints/Enums/E_RuneType Enum" :default "NewEnumerator0"))
  (returns (`Empty?` :type Boolean) (Widget :type "/Game/RunesSystem/Widgets/WBP_Rune Object Reference"))
  ;[0 0 0] Check if there is an empty rune, so you can return the rune back to it's original slot
  (bind _foundwidgets (`WidgetBlueprintLibrary.GetAllWidgetsOfClass` null "/Game/RunesSystem/Widgets/WBP_MainWidget.WBP_MainWidget_C" false))
  (for _array_element (`/Game/RunesSystem/Widgets/WBP_MainWidget.AllRuneWidgets` (`|GetArrayItem` _foundwidgets))
    (if (`|EnumEquality` (`local.RuneType`) (`/Game/RunesSystem/Widgets/WBP_Rune.RuneType_Permanent` _array_element))
      (if (not (`self.IsValidRune` (`.RuneID_8_2826BC2F4E2640B16668778B80A6A69C` (break `/Game/RunesSystem/Blueprints/Structures/ST_Rune` (`/Game/RunesSystem/Widgets/WBP_Rune.RuneInfo` _array_element)))))
        (return true _array_element))))
  (return false null))

(fn `GetEmptyRuneSlot`
  (params (RuneToPlace :type "/Game/RunesSystem/Widgets/WBP_Rune Object Reference"))
  (returns (`Found?` :type Boolean) (Widget :type "/Game/RunesSystem/Widgets/WBP_RuneSlot Object Reference"))
  ;[0 0 0] Check if there is an empty rune slot that meets the requirements
  (bind _foundwidgets (`WidgetBlueprintLibrary.GetAllWidgetsOfClass` null "/Game/RunesSystem/Widgets/WBP_MainWidget.WBP_MainWidget_C" false))
  (for _array_element (`/Game/RunesSystem/Widgets/WBP_MainWidget.GetAllRuneSlots` (`|GetArrayItem` _foundwidgets))
    (bind _level (message `/Game/RunesSystem/Blueprints/BP_BPI_RuneSystem.GetPlayerLevel` (`GameplayStatics.GetPlayerCharacter` null)))
    (if (and (not (`self.IsValidRune` (`.RuneID_8_2826BC2F4E2640B16668778B80A6A69C` (break `/Game/RunesSystem/Blueprints/Structures/ST_Rune` (`/Game/RunesSystem/Widgets/WBP_RuneSlot.Rune` _array_element))))) (`self.LevelRequirement` _level (`/Game/RunesSystem/Widgets/WBP_RuneSlot.RequiredLevel` _array_element)) (`|EnumEquality` (`/Game/RunesSystem/Widgets/WBP_RuneSlot.RuneSlotType` _array_element) (`.RuneType_30_09802FE345743C7375BE12A46FFBC4AF` (break `/Game/RunesSystem/Blueprints/Structures/ST_Rune` (`/Game/RunesSystem/Widgets/WBP_Rune.RuneInfo` (`local.RuneToPlace`))))))
      (return true _array_element)))
  (return false null))

(fn `GetPlayerCharacter`
  (returns (PlayerCharacter :type "/Game/RunesSystem/Blueprints/BP_RuneCharacter Object Reference"))
  (bind _asbp_rune_character (cast `/Game/RunesSystem/Blueprints/BP_RuneCharacter` (`GameplayStatics.GetPlayerCharacter` null)))
  (return _asbp_rune_character))

(fn `GetRuneTypeColor`
  (params (RuneType :type "/Game/RunesSystem/Blueprints/Enums/E_RuneType Enum" :default "NewEnumerator0"))
  (returns (ReturnValue :type "LinearColor Structure"))
  (return (select `/Game/RunesSystem/Blueprints/Enums/E_RuneType` RuneType :`NewEnumerator0` (struct :`R` 0.097587 :`G` 0.088656 :`B` 0.099899 :`A` 1.0) :`NewEnumerator1` (struct :`R` 0.040915 :`G` 0.300544 :`B` 0.012286 :`A` 1.0) :`NewEnumerator4` (struct :`R` 0.198069 :`G` 0.000911 :`B` 0.015996 :`A` 1.0) :`NewEnumerator2` (struct :`R` 0.300544 :`G` 0.012983 :`B` 0.603828 :`A` 1.0) :!type "LinearColor Structure")))

(fn `GetSpiritFormulaType`
  (returns (Type :type "/Game/RunesSystem/Blueprints/Enums/E_FormulaType Enum"))
  (return "NewEnumerator0"))

(fn `IsValidRune`
  (params (Rune :type Name))
  (returns (`Valid?` :type Boolean))
  (bind ((`RuneID_8_2826BC2F4E2640B16668778B80A6A69C` _runeid) (`Icon_4_971A931C4E98C79372C75CBC9723B082` _icon) (`Stats_16_EC13C11D4FC3E734A4469B91A9968DB2` _stats)) (break `/Game/RunesSystem/Blueprints/Structures/ST_Rune` (`self.GetDatatableRune` Rune)))
  (return (and (!= _runeid "None") (`KismetSystemLibrary.IsValid` _icon) (> (`KismetArrayLibrary.Array_Length` _stats) 0))))

(fn `LevelRequirement`
  (params (PlayerLevel :type Integer) (RequiredLevel :type Integer))
  (returns (Out :type Boolean))
  (return (>= PlayerLevel RequiredLevel)))

(fn `RuneIsAMatch`
  (params (RuneTypes :type "Array of /Game/RunesSystem/Blueprints/Enums/E_RuneType Enum") (CompareTo :type "/Game/RunesSystem/Blueprints/Enums/E_RuneType Enum" :default "NewEnumerator0"))
  (returns (Out :type Boolean))
  (for _array_element RuneTypes
    (if (`|EnumEquality` _array_element (`local.CompareTo`))
      (return true))))