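; Main_Serath_BP is the Serath character Blueprint, handling a brief camera cut-in during critical attacks.
; Tick watches the CriticalAttack flag and, through a DoOnce, switches FollowCamera to the face anchor, then back to the main boom after a short delay.
; SwitchCamera reparents the camera to the component chosen by CamType, keeping world transform, then eases it into place with MoveComponentTo.
; The Legs view has no component assigned.
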(event `self.SwitchCamera`
  (params (CamType :type "/Game/MainCharacter/Enum_CamType Enum" :default "NewEnumerator0") (Cam :type "CameraComponent Object Reference"))
  (`SceneComponent.K2_AttachToComponent` Cam (select `/Game/MainCharacter/Enum_CamType` CamType :`NewEnumerator0` (`self.CameraBoom`) :`NewEnumerator1` (`self.SA_Face`) :!type "SceneComponent Object Reference") "None" "KeepWorld" "KeepWorld" "KeepWorld" true)
  (`KismetSystemLibrary.MoveComponentTo` Cam (0.0 0.0 0.0) (struct) true true 0.4 true))

(event `self.ReceiveTick`
  (params (DeltaSeconds :type "Float (single-precision)"))
  (if (`self.bCriticalAttack`)
    (`/Engine/EditorBlueprintResources/StandardMacros.DoOnce` false :!label _label
      (:`Completed`
        (`self.SwitchCamera` "NewEnumerator1" (`self.FollowCamera`))
        (`KismetSystemLibrary.Delay` 1.2)
        (`self.SwitchCamera` "NewEnumerator0" (`self.FollowCamera`))
        (goto _label :!via `Reset`)))))

(fn `UserConstructionScript`)